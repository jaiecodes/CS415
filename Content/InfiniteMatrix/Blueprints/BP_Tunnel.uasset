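; Endless-runner tunnel segment with a rotating holed wall that damages the player on contact and triggers the restart display at low health.
; Its end trigger spawns the next tunnel, scores unhit passes, and destroys itself with its pickup and enemy.
; A one-shot trigger randomly spawns both ahead, offsetting enemy coordinates against a re-rolled pack position, not the actual one.
; RandomizeWall, uncalled here, picks mesh and roll.
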(event OnComponentBeginOverlap(TriggerZone)
  (params (OverlappedComponent :type Primitive%20Component%20Object%20Reference) (OtherActor :type Actor%20Object%20Reference) (OtherComp :type Primitive%20Component%20Object%20Reference) (OtherBodyIndex :type Integer) (bFromSweep :type Boolean) (SweepResult :type Hit%20Result%20Structure%20%28by%20ref%29))
  (bind _lasthealthpack (Variables|Default|GetLastHealthPack))
  (bind _lastenemy (Variables|Default|GetLastEnemy))
  (bind _asbp_player (Utilities|Casting|CastToBP_Player OtherActor))
  (Default|SpawnTunnelatSpawnPoint (Variables|Default|GetTunnelSpawner))
  (Actor|DestroyActor)
  (if (Variables|Default|GetbWasHit)
    _
    (else
      (Default|UpdateScore _asbp_player)))
  (Variables|Default|SetbWasHit false)
  (Utilities|IsValid _lasthealthpack
    (:Is%20Valid
      (Actor|DestroyActor _lasthealthpack))
    (:Is%20Not%20Valid
      _))
  (Utilities|IsValid _lastenemy
    (:Is%20Valid
      (Actor|DestroyActor _lastenemy))))

(event OnComponentBeginOverlap(WallMesh)
  (params (OverlappedComponent :type Primitive%20Component%20Object%20Reference) (OtherActor :type Actor%20Object%20Reference) (OtherComp :type Primitive%20Component%20Object%20Reference) (OtherBodyIndex :type Integer) (bFromSweep :type Boolean) (SweepResult :type Hit%20Result%20Structure%20%28by%20ref%29))
  (bind _asbp_player (Utilities|Casting|CastToBP_Player OtherActor))
  (Default|UpdateHealth _asbp_player false)
  (bind _currhealth (Default|GetHealth _asbp_player))
  (if (> _currhealth 0.2)
    (Variables|Default|SetbWasHit true)
    (else
      (Variables|/Game/InfiniteMatrix/Blueprints/BP_Player.BP_Player_C|SetIsDead _asbp_player true)
      (Default|DisplayRestart _asbp_player))))

(event OnComponentBeginOverlap(HealthPackTrigger)
  (params (OverlappedComponent :type Primitive%20Component%20Object%20Reference) (OtherActor :type Actor%20Object%20Reference) (OtherComp :type Primitive%20Component%20Object%20Reference) (OtherBodyIndex :type Integer) (bFromSweep :type Boolean) (SweepResult :type Hit%20Result%20Structure%20%28by%20ref%29))
  (Utilities|FlowControl|DoOnce false
    (:Completed
      (bind _packlocation (CallFunction|SpawnHealthPack))
      (CallFunction|SpawnEnemy _packlocation))))

(event EventBeginPlay)

(event EventTick
  (params (DeltaSeconds :type Float%20%28single-precision%29))
  (Transformation|AddLocalRotation (Variables|Default|GetWallMesh) (Math|Rotator|MakeRotator (* DeltaSeconds (Variables|Default|GetRotateSpeed)) 0.0 0.0) false false))

(fn ConstructionScript)

(fn RandomizeWall
  (Components|StaticMesh|SetStaticMesh (Variables|Default|GetWallMesh) (Utilities|Select :Index (Math|Random|RandomIntegerinRange 0 3) :Option%200 "/Game/InfiniteMatrix/Meshes/SM_Hole_01.SM_Hole_01" :Option%201 "/Game/InfiniteMatrix/Meshes/SM_Hole_02.SM_Hole_02" :Option%202 "/Game/InfiniteMatrix/Meshes/SM_Hole_03.SM_Hole_03" :Option%203 "/Game/InfiniteMatrix/Meshes/SM_Hole_04.SM_Hole_04"))
  (Transformation|AddLocalRotation (Variables|Default|GetWallMesh) (Math|Rotator|MakeRotator (Math|Random|RandomFloatinRange 0.0 3.6e+02) 0.0 0.0) false false))

(fn SpawnHealthPack
  (bind _returnvalue (Math|Random|RandomFloatinRange -1.5e+02 1.5e+02))
  (bind _returnvalue_2 (Math|Random|RandomFloatinRange -1.5e+02 1.5e+02))
  (bind _healthpacktrigger (Variables|Default|GetHealthPackTrigger))
  (bind _returnvalue_3 (Transformation|GetWorldLocation _healthpacktrigger))
  (bind _returnvalue_4 (+ (.x _returnvalue_3) 7.5e+02))
  (bind _returnvalue_5 (+ (.x _returnvalue_3) 2e+03))
  (bind _returnvalue_6 (Math|Random|RandomFloatinRange _returnvalue_4 _returnvalue_5))
  (bind _returnvalue_7 (Math|Vector|MakeVector _returnvalue_6 _returnvalue_2 _returnvalue))
  (if (Math|Random|RandomBoolwithWeight 0.55)
    (bind _returnvalue_8 (Game|SpawnActorfromClass "/Game/InfiniteMatrix/Blueprints/BP_HealthPack.BP_HealthPack_C" (Math|Transform|MakeTransform _returnvalue_7 "0, 0, 0" "1.000000,1.000000,1.000000") "Undefined" "MultiplyWithRoot" 0 0))
    (Variables|Default|SetLastHealthPack _returnvalue_8)
    (return _returnvalue_7)))

(fn SpawnEnemy
  (params (PackLocation :type Vector))
  (bind _healthpacktrigger (Variables|Default|GetHealthPackTrigger))
  (bind _returnvalue (Transformation|GetWorldLocation _healthpacktrigger))
  (if (Math|Random|RandomBoolwithWeight 0.8)
    (bind _newpos (CallFunction|CheckRange (Math|Random|RandomFloatinRange (+ (.x _returnvalue) 8.6e+02) (+ (.x _returnvalue) 2e+03)) (.x PackLocation) 75.0))
    (bind _newpos_2 (CallFunction|CheckRange (Math|Random|RandomFloatinRange -1.5e+02 1.5e+02) (.y PackLocation) 75.0))
    (bind _newpos_3 (CallFunction|CheckRange (Math|Random|RandomFloatinRange -1.5e+02 1.5e+02) (.z PackLocation) 75.0))
    (bind _returnvalue_2 (Game|SpawnActorfromClass "/Game/InfiniteMatrix/Blueprints/BP_Enemies.BP_Enemies_C" (Math|Transform|MakeTransform (Math|Vector|MakeVector _newpos _newpos_2 _newpos_3) "0, 0, 0" "1.000000,1.000000,1.000000") "AlwaysSpawn" "MultiplyWithRoot" 0 0))
    (Variables|Default|SetLastEnemy _returnvalue_2)))

(fn CheckRange
  (params (Pos :type Float%20%28double-precision%29) (TargetPos :type Float%20%28double-precision%29) (Range :type Float%20%28double-precision%29))
  (if (or (<= (+ TargetPos Range) Pos) (>= Pos (- TargetPos Range)))
    (return (+ Pos 5e+01))
    (else
      (return Pos))))